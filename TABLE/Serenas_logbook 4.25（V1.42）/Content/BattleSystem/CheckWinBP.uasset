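; CheckWinBP is a battle-system actor that decides when a fight is won or lost.
; CheckWinEvent receives an actor, identifies it as enemy or friendly, and treats it as the side's last if only one of that class exists.
; It then shows a BattleEnd widget and destroys itself.
; On a win, it also passes reward, return-teleport and mission/chapter data to the widget's CloseLevelWG.
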(event Custom|CheckWinEvent
  (params (Actor :type Actor%20Object%20Reference))
  (Utilities|Casting|CastToEnemyActor Actor
    (:then
      (bind _outactors (Actor|GetAllActorsOfClass "/Game/HeroBP/BattleActor/EnemyActor.EnemyActor_C"))
      (if (== (Utilities|Array|Length _outactors) 1)
        (bind _returnvalue (UserInterface|CreateWidget "/Game/UMG/BattleUI/LevelBeginWG/CheckWinWG/BattleEnd.BattleEnd_C" 0 true))
        (Variables|/Game/UMG/BattleUI/LevelBeginWG/CheckWinWG/CloseLevelWG.CloseLevelWG_C|SetExp (Variables|/Game/UMG/BattleUI/LevelBeginWG/CheckWinWG/BattleEnd.BattleEnd_C|GetCloseLevelWG _returnvalue) (Variables|Default|GetEXP))
        (Variables|/Game/UMG/BattleUI/LevelBeginWG/CheckWinWG/CloseLevelWG.CloseLevelWG_C|SetLevel (Variables|/Game/UMG/BattleUI/LevelBeginWG/CheckWinWG/BattleEnd.BattleEnd_C|GetCloseLevelWG _returnvalue) (Variables|Default|GetLevel))
        (Variables|/Game/UMG/BattleUI/LevelBeginWG/CheckWinWG/CloseLevelWG.CloseLevelWG_C|SetTeleportLocation (Variables|/Game/UMG/BattleUI/LevelBeginWG/CheckWinWG/BattleEnd.BattleEnd_C|GetCloseLevelWG _returnvalue) (Variables|Default|GetReturnLocation))
        (Variables|/Game/UMG/BattleUI/LevelBeginWG/CheckWinWG/CloseLevelWG.CloseLevelWG_C|SetTeleportMap (Variables|/Game/UMG/BattleUI/LevelBeginWG/CheckWinWG/BattleEnd.BattleEnd_C|GetCloseLevelWG _returnvalue) (Variables|Default|GetReturnMap))
        (Variables|/Game/UMG/BattleUI/LevelBeginWG/CheckWinWG/CloseLevelWG.CloseLevelWG_C|SetMainMission (Variables|/Game/UMG/BattleUI/LevelBeginWG/CheckWinWG/BattleEnd.BattleEnd_C|GetCloseLevelWG _returnvalue) (Variables|Default|GetMainMission))
        (Variables|/Game/UMG/BattleUI/LevelBeginWG/CheckWinWG/CloseLevelWG.CloseLevelWG_C|SetChapter (Variables|/Game/UMG/BattleUI/LevelBeginWG/CheckWinWG/BattleEnd.BattleEnd_C|GetCloseLevelWG _returnvalue) (Variables|Default|GetChapter))
        (UserInterface|Viewport|AddtoViewport _returnvalue 0)
        (Actor|DestroyActor :!label _label)))
    (:CastFailed
      (Utilities|Casting|CastToFriendlyActor Actor)
      (bind _outactors_2 (Actor|GetAllActorsOfClass "/Game/HeroBP/BattleActor/FriendlyActor.FriendlyActor_C"))
      (if (== (Utilities|Array|Length _outactors_2) 1)
        (bind _returnvalue_2 (UserInterface|CreateWidget "/Game/UMG/BattleUI/LevelBeginWG/CheckWinWG/BattleEnd.BattleEnd_C"))
        (UserInterface|Viewport|AddtoViewport _returnvalue_2 0)
        (goto _label)))))

(event EventBeginPlay)

(event Collision|EventActorBeginOverlap
  (params (OtherActor :type Actor%20Object%20Reference)))

(event EventTick
  (params (DeltaSeconds :type Float%20%28single-precision%29)))

(fn ConstructionScript)