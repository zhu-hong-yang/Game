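; FireBP is a battle-system world object, apparently a fire effect, that billboards its Scene component toward the player camera.
; Every Tick it takes the look-at rotation to the camera and applies the yaw with a 90-degree offset.
; The look-at pitch is remapped into a clamped roll, so it tilts at most 20 degrees toward a higher camera and stays upright for a lower one.
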(event EventBeginPlay)

(event Collision|EventActorBeginOverlap
  (params (OtherActor :type Actor%20Object%20Reference)))

(event EventTick
  (params (DeltaSeconds :type Float%20%28single-precision%29))
  (bind _returnvalue (Game|GetPlayerCameraManager 0))
  (bind _scene (Variables|Default|GetScene))
  (bind _returnvalue_2 (Transformation|GetWorldLocation _scene))
  (bind _returnvalue_3 (Camera|GetCameraLocation _returnvalue))
  (bind _returnvalue_4 (Math|Rotator|FindLookatRotation _returnvalue_2 _returnvalue_3))
  (bind (_roll _pitch _yaw) (Math|Rotator|BreakRotator _returnvalue_4))
  (Transformation|SetWorldRotation (Variables|Default|GetScene) (Math|Rotator|MakeRotator (Math|Float|Clamp(Float) (- 3.6e+02 _pitch) 3.4e+02 3.6e+02) 0.0 (- _yaw 9e+01)) false false))

(fn ConstructionScript)