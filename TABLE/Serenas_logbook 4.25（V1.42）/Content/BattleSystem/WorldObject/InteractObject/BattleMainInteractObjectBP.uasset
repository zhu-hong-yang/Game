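; Base battle world interact object that reports its movement to the game state and affects heroes it hits.
; UpdateInteractObject raises InteractObjectMoving on BattleGameState, then polls velocity on a short delay loop and clears the flag shortly after reading zero.
; Hit sends a stun interact message to the other actor's HeroStatComponent, when present.
; Destruction also clears the moving flag.
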(event EventDestroyed
  (bind _asbattle_game_state (Utilities|Casting|CastToBattleGameState (Game|GetGameState)))
  (Variables|/Game/PlayerInfo/BattleMode/BattleGameState.BattleGameState_C|SetInteractObjectMoving _asbattle_game_state false))

(event Collision|EventHit
  (params (MyComp :type Primitive%20Component%20Object%20Reference) (Other :type Actor%20Object%20Reference) (OtherComp :type Primitive%20Component%20Object%20Reference) (bSelfMoved :type Boolean) (HitLocation :type Vector :default "0, 0, 0") (HitNormal :type Vector :default "0, 0, 0") (NormalImpulse :type Vector :default "0, 0, 0") (Hit :type Hit%20Result%20Structure%20%28by%20ref%29))
  (bind _returnvalue (Actor|GetComponentbyClass Other "/Game/HeroBP/BattleActor/HeroStatComponent.HeroStatComponent_C"))
  (Utilities|IsValid _returnvalue
    (:Is%20Valid
      (Class|SLGInteractInterface|SLGStunInteract(Message) _returnvalue self))))

(event EventUpdateInteractObject
  (bind _asbattle_game_state (Utilities|Casting|CastToBattleGameState (Game|GetGameState)))
  (Variables|/Game/PlayerInfo/BattleMode/BattleGameState.BattleGameState_C|SetInteractObjectMoving _asbattle_game_state true)
  (Utilities|FlowControl|Delay 0.2 :!label _label)
  (if (== (Math|Vector|VectorLength (Transformation|GetVelocity)) 0.0)
    (Utilities|FlowControl|Delay 1.0)
    (Variables|/Game/PlayerInfo/BattleMode/BattleGameState.BattleGameState_C|SetInteractObjectMoving _asbattle_game_state false)
    (else
      (goto _label))))

(fn ConstructionScript)