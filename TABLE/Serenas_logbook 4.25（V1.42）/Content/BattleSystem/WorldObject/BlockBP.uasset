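; Grid terrain block for SLG battles that carries ground type and spreading Poison/Fire damage-over-time states.
; Items or neighbouring blocks apply states by ground type: grass accepts both, dry ground only poison, tinting materials and spawning fire.
; GameState-registered blocks age states each round, spreading them by line traces; expired fire leaves dry ground.
; Construction sets per-face textures, marks walls and water as obstacles, and hides trace-detected covered faces.
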(event Custom|BlockAddDOT_Event
  (params (BlockBP :type Block%20BP%20Object%20Reference%20%28by%20ref%29) (ItemToFind :type E_DOT_Type%20Enum%20%28by%20ref%29 :default "NewEnumerator18"))
  (bind _returnvalue (Transformation|GetActorTransform))
  (bind _self self)
  (bind (_location _rotation _scale) (Math|Transform|BreakTransform _returnvalue))
  ;[1 1 1] 添加状态
  (switch Utilities|FlowControl|Switch|SwitchonE_GroundName (Variables|Default|GetE_GroundName)
    (:NewEnumerator0
      (switch Utilities|FlowControl|Switch|SwitchonE_DOT_Type ItemToFind
        (:NewEnumerator18
          (for _array_element (Variables|Default|GetDynamicMatArray) :!label _label
            (Rendering|Material|SetVectorParameterValue _array_element "BlockColor" (Variables|毒|GetPoisonColor) :!class /Script/Engine.MaterialInstanceDynamic))
          (if (== BlockBP _self)
            (Variables|毒|SetPoisonRoundNow 0)
            (else
              (Variables|毒|SetPoisonRoundNow (Variables|毒|GetPoisonRoundNow _self)))))
        (:NewEnumerator19
          (bind _returnvalue_2 (Game|SpawnActorfromClass "/Game/BattleSystem/WorldObject/FireBP.FireBP_C" (Math|Transform|MakeTransform (+ _location "0.000000, 0,40.000000") _rotation _scale) "AdjustIfPossibleButAlwaysSpawn" 0 0))
          (Variables|Default|SetRefFireBP _returnvalue_2)
          (for _array_element_2 (Variables|Default|GetDynamicMatArray)
            (Rendering|Material|SetVectorParameterValue _array_element_2 "BlockColor" (Variables|火|GetFireColor) :!class /Script/Engine.MaterialInstanceDynamic))
          (Variables|火|SetFireRoundNow 0))))
    (:NewEnumerator1
      (switch Utilities|FlowControl|Switch|SwitchonE_DOT_Type ItemToFind
        (:NewEnumerator18
          (goto _label))))))

(event Custom|CheckAroundBlockEvent
  (params (Index :type E_DOT_Type%20Enum :default "NewEnumerator18"))
  (bind _returnvalue (Transformation|GetActorLocation))
  ;[1 1 1] 检测和给予附近格子状态
  (for (_array_element _array_index) (Utilities|Select :Index Index :NewEnumerator18 (Utilities|Array|MakeArray "100.000000,0.000000,-40.000000" "-100.000000,0.000000,-40.000000" "0.000000,100.000000,-40.000000" "0.000000,-100.000000,-40.000000" "0.000000,0.000000,-110.000000" "0.000000,100.000000,-110.000000" "0.000000,-100.000000,-110.000000" "100.000000,0.000000,-110.000000" "-100.000000,0.000000,-110.000000") :NewEnumerator19 (Utilities|Array|MakeArray "100.000000,0.000000,40.000000" "-100.000000,0.000000,40.000000" "0.000000,100.000000,40.000000" "0.000000,-100.000000,40.000000" "0.000000,0.000000,110.000000" "0.000000,100.000000,110.000000" "0.000000,-100.000000,110.000000" "100.000000,0.000000,110.000000" "-100.000000,0.000000,110.000000"))
    (bind (_outhit _returnvalue_2) (Collision|LineTraceForObjects (+ _returnvalue (select (== _array_index 8) "0, 0, 0" (Math|Vector|MakeVector 0.0 0.0 (.Z (Math|Vector|BreakVector _array_element))))) (+ _returnvalue _array_element) (Utilities|Array|MakeArray "ObjectTypeQuery8") false 0 "None"))
    (if _returnvalue_2
      (Class|SLGBlockInterface|SLGBlockInteract(Message) (.HitActor (Collision|BreakHitResult _outhit)) (Utilities|Map|MakeMap self Index)))))

(event EventBeginPlay
  (bind _box (Variables|Default|GetBox))
  ;[1 1 1] 初始化格子
  (Collision|SetCollisionResponsetoChannel _box "ECC_GameTraceChannel5" (select (Variables|Default|GetBlockObject) "ECR_Block" "ECR_Ignore"))
  (Collision|SetCollisionObjectType _box "ECC_GameTraceChannel3")
  (Utilities|Map|Clear (Variables|Default|GetCheckRefP_Block)))

(event EventSLGRoundBeginUpdate
  (bind _poisonspillround (Variables|毒|GetPoisonSpillRound))
  ;[1 1 1] 每回合开始更新
  (bind (_arrayindex _arrayelement) (Utilities|Array|ReverseforEachLoop (Variables|Default|GetDOT_DamageType))
    (:LoopBody
      (switch Utilities|FlowControl|Switch|SwitchonE_DOT_Type _arrayelement
        (:NewEnumerator18
          (Variables|毒|SetPoisonRoundNow (+ (Variables|毒|GetPoisonRoundNow) 1))
          (if (> (Variables|毒|GetPoisonRoundNow) (Variables|毒|GetPoisonMaxRound))
            (Utilities|Array|RemoveIndex (Variables|Default|GetDOT_DamageType) _arrayindex :!label _label)
            (elif (not (Variables|毒|GetPoisonSpillDone))
              (if (== (Class|KismetMathLibrary|PercentByteByte (Variables|毒|GetPoisonRoundNow) _poisonspillround) 0)
                (if (<= (/ (Variables|毒|GetPoisonRoundNow) _poisonspillround) (Variables|毒|GetPoisonMaxSpill))
                  (Variables|毒|SetPoisonSpillDone true)
                  (CallFunction|CheckAroundBlockEvent "NewEnumerator18"))))))
        (:NewEnumerator19
          (Variables|火|SetFireRoundNow (+ (Variables|火|GetFireRoundNow) 1))
          (if (> (Variables|火|GetFireRoundNow) (Variables|火|GetFireMaxRound))
            (Actor|DestroyActor (Variables|Default|GetRefFireBP))
            (CallFunction|SetupBlockTexture "NewEnumerator1")
            (for _array_element (Variables|Default|GetDynamicMatArray)
              (Rendering|Material|SetVectorParameterValue _array_element "BlockColor" (Variables|默认|GetNormalColor) :!class /Script/Engine.MaterialInstanceDynamic))
            (goto _label)
            (elif (not (Variables|火|GetFireSpillDone))
              (if (== (Class|KismetMathLibrary|PercentByteByte (Variables|火|GetFireRoundNow) (Variables|火|GetFireSpillRound)) 0)
                (Variables|火|SetFireSpillDone true)
                (CallFunction|CheckAroundBlockEvent "NewEnumerator19")))))))
    (:Completed
      (if (== (Utilities|Array|Length (Variables|Default|GetDOT_DamageType)) 0)
        (Class|SLGInteractInterface|SLGAddandRemoveActorArrayInteract(Message) (Game|GetGameState) self false)))))

(event EventSLGUseItem
  ;[1 1 1] 使用道具
  ;[1 1 1] 判定什么状态可添加
  (bind _values (Utilities|Map|Values (Variables|Default|GetCheckRefP_Block)))
  (Variables|Default|SetCheckBool false)
  (for (_array_element _array_index) _values
    (if (not (Utilities|Array|ContainsItem (Variables|Default|GetDOT_DamageType) _array_element))
      (switch Utilities|FlowControl|Switch|SwitchonE_GroundName (Variables|Default|GetE_GroundName)
        (:NewEnumerator0
          (switch Utilities|FlowControl|Switch|SwitchonE_DOT_Type _array_element
            (:NewEnumerator18
              _)
            (:NewEnumerator19
              _)))
        (:NewEnumerator1
          (switch Utilities|FlowControl|Switch|SwitchonE_DOT_Type _array_element
            (:NewEnumerator18
              _))))
      (Variables|Default|SetCheckBool true)
      (bind _keys (Utilities|Map|Keys (stale EventSLGBlockInteract P_Block)))
      (CallFunction|BlockAddDOTEvent (Utilities|Array|Get(acopy) _keys _array_index) _array_element)
      (Utilities|Array|AddUnique (Variables|Default|GetDOT_DamageType) _array_element)))
  (if (Variables|Default|GetCheckBool)
    (Class|SLGInteractInterface|SLGAddandRemoveActorArrayInteract(Message) (Game|GetGameState) self true)))

(event EventSLGBlockInteract
  (params (P_Block :type Map%20of%20Block%20BP%20Object%20References%20to%20Bytes))
  ;[1 1 1] 判定什么状态可添加
  (Variables|Default|SetCheckRefP_Block P_Block)
  (bind _values (Utilities|Map|Values (Variables|Default|GetCheckRefP_Block)))
  (Variables|Default|SetCheckBool false)
  (for (_array_element _array_index) _values
    (if (not (Utilities|Array|ContainsItem (Variables|Default|GetDOT_DamageType) _array_element))
      (switch Utilities|FlowControl|Switch|SwitchonE_GroundName (Variables|Default|GetE_GroundName)
        (:NewEnumerator0
          (switch Utilities|FlowControl|Switch|SwitchonE_DOT_Type _array_element
            (:NewEnumerator18
              _)
            (:NewEnumerator19
              _)))
        (:NewEnumerator1
          (switch Utilities|FlowControl|Switch|SwitchonE_DOT_Type _array_element
            (:NewEnumerator18
              _))))
      (Variables|Default|SetCheckBool true)
      (bind _keys (Utilities|Map|Keys P_Block))
      (CallFunction|BlockAddDOTEvent (Utilities|Array|Get(acopy) _keys _array_index) _array_element)
      (Utilities|Array|AddUnique (Variables|Default|GetDOT_DamageType) _array_element)))
  (if (Variables|Default|GetCheckBool)
    (Class|SLGInteractInterface|SLGAddandRemoveActorArrayInteract(Message) (Game|GetGameState) self true)))

(fn ConstructionScript
  (bind _returnvalue (Transformation|GetActorLocation))
  (Utilities|FlowControl|Sequence
    (:then_0
      (CallFunction|BeginSetupBlockTexture))
    (:then_1
      (switch Utilities|FlowControl|Switch|SwitchonE_GroundName (Variables|Default|GetE_GroundName)
        (:NewEnumerator0
          (Variables|Default|SetBlockObject false :!label _label))
        (:NewEnumerator1
          (goto _label))
        (:NewEnumerator2
          (Variables|Default|SetBlockObject true :!label _label_2))
        (:NewEnumerator3
          (goto _label_2))))
    (:then_2
      (for (_array_element _array_index) (Utilities|Array|MakeArray "100.000000, 0,40.000000" "-100.000000,0.000000,40.000000" "0.000000,100.000000,40.000000" "0.000000,-100.000000,40.000000" "0, 0,100.000000")
        (bind (_outhit _returnvalue_2) (Collision|LineTraceForObjects (+ _returnvalue "0, 0,40.000000") (+ _returnvalue (Math|Vector|RotateVector _array_element (Transformation|GetActorRotation))) (Utilities|Array|MakeArray "ObjectTypeQuery8") false 0 "None"))
        (if _returnvalue_2
          (Rendering|SetVisibility (Utilities|Array|Get(acopy) (Utilities|Array|MakeArray (Variables|Default|GetRightPlane) (Variables|Default|GetLeftPlane) (Variables|Default|GetBackPlane) (Variables|Default|GetFrontPlane) (Variables|Default|GetTopPlane)) _array_index) false false))))))

(fn BeginSetupBlockTexture
  (bind _e_groundname (Variables|Default|GetE_GroundName))
  (bind _groundtexturemapping (Variables|Default|GetGroundTextureMapping))
  (bind _dynamicmatarray (Variables|Default|GetDynamicMatArray))
  (bind _value (Utilities|Map|Find _groundtexturemapping _e_groundname))
  (Utilities|FlowControl|Sequence
    (:then_0
      (bind _returnvalue (Rendering|Material|CreateDynamicMaterialInstance (Variables|Default|GetTopPlane) 0 "/Game/BattleSystem/Box_Mat_Inst.Box_Mat_Inst" "None" :!class /Script/Engine.PrimitiveComponent))
      (Utilities|Array|SetArrayElem _dynamicmatarray 0 _returnvalue true)
      (Rendering|Material|SetTextureParameterValue _returnvalue "MyTexture" _value))
    (:then_1
      (bind _returnvalue_2 (Rendering|Material|CreateDynamicMaterialInstance (Variables|Default|GetLeftPlane) 0 "/Game/BattleSystem/Box_Mat_Inst.Box_Mat_Inst" "None" :!class /Script/Engine.PrimitiveComponent))
      (Utilities|Array|SetArrayElem _dynamicmatarray 1 _returnvalue_2 true)
      (Rendering|Material|SetTextureParameterValue _returnvalue_2 "MyTexture" _value))
    (:then_2
      (bind _returnvalue_3 (Rendering|Material|CreateDynamicMaterialInstance (Variables|Default|GetFrontPlane) 0 "/Game/BattleSystem/Box_Mat_Inst.Box_Mat_Inst" "None" :!class /Script/Engine.PrimitiveComponent))
      (Utilities|Array|SetArrayElem _dynamicmatarray 2 _returnvalue_3 true)
      (Rendering|Material|SetTextureParameterValue _returnvalue_3 "MyTexture" _value))
    (:then_3
      (bind _returnvalue_4 (Rendering|Material|CreateDynamicMaterialInstance (Variables|Default|GetRightPlane) 0 "/Game/BattleSystem/Box_Mat_Inst.Box_Mat_Inst" "None" :!class /Script/Engine.PrimitiveComponent))
      (Utilities|Array|SetArrayElem _dynamicmatarray 3 _returnvalue_4 true)
      (Rendering|Material|SetTextureParameterValue _returnvalue_4 "MyTexture" _value))
    (:then_4
      (bind _returnvalue_5 (Rendering|Material|CreateDynamicMaterialInstance (Variables|Default|GetBackPlane) 0 "/Game/BattleSystem/Box_Mat_Inst1.Box_Mat_Inst1" "None" :!class /Script/Engine.PrimitiveComponent))
      (Utilities|Array|SetArrayElem _dynamicmatarray 4 _returnvalue_5 true)
      (Rendering|Material|SetTextureParameterValue _returnvalue_5 "MyTexture" _value)
      (return))))

(fn SetupBlockTexture
  (params (GroundName :type E_GroundName%20Enum :default "NewEnumerator0"))
  (bind _dynamicmatarray (Variables|Default|GetDynamicMatArray))
  (Variables|Default|SetE_GroundName GroundName)
  (Utilities|FlowControl|Sequence
    (:then_0
      (Rendering|Material|SetTextureParameterValue (Utilities|Array|Get(acopy) _dynamicmatarray) "MyTexture" (.Value (Utilities|Map|Find (Variables|Default|GetGroundTextureMapping) (Variables|Default|GetE_GroundName)))))
    (:then_1
      (Rendering|Material|SetTextureParameterValue (Utilities|Array|Get(acopy) _dynamicmatarray 1) "MyTexture" (.Value (Utilities|Map|Find (Variables|Default|GetGroundTextureMapping) (Variables|Default|GetE_GroundName)))))
    (:then_2
      (Rendering|Material|SetTextureParameterValue (Utilities|Array|Get(acopy) _dynamicmatarray 2) "MyTexture" (.Value (Utilities|Map|Find (Variables|Default|GetGroundTextureMapping) (Variables|Default|GetE_GroundName)))))
    (:then_3
      (Rendering|Material|SetTextureParameterValue (Utilities|Array|Get(acopy) _dynamicmatarray 3) "MyTexture" (.Value (Utilities|Map|Find (Variables|Default|GetGroundTextureMapping) (Variables|Default|GetE_GroundName)))))
    (:then_4
      (Rendering|Material|SetTextureParameterValue (Utilities|Array|Get(acopy) _dynamicmatarray 4) "MyTexture" (.Value (Utilities|Map|Find (Variables|Default|GetGroundTextureMapping) (Variables|Default|GetE_GroundName))))
      (return))))

(fn SLGCheckCanUseItem
  (params (MainGoodsStatSt :type Main%20Item%20St%20Structure))
  (bind _dot (Utilities|Struct|BreakMainItemSt MainGoodsStatSt))
  (Utilities|Map|Clear (Variables|Default|GetCheckRefP_Block))
  (bind _values (Utilities|Map|Values _dot))
  (bind _keys (Utilities|Map|Keys _dot))
  (for (_ _array_index) _values
    (switch Utilities|FlowControl|Switch|SwitchonE_GroundName (Variables|Default|GetE_GroundName)
      (:NewEnumerator0
        (switch Utilities|FlowControl|Switch|SwitchonE_DOT_Type (Utilities|Array|Get(acopy) _keys _array_index)
          (:NewEnumerator18
            _)
          (:NewEnumerator19
            _)))
      (:NewEnumerator1
        (switch Utilities|FlowControl|Switch|SwitchonE_DOT_Type (Utilities|Array|Get(acopy) _keys _array_index)
          (:NewEnumerator18
            _))))
    (Utilities|Map|Add (Variables|Default|GetCheckRefP_Block) self (Utilities|Array|Get(acopy) _keys _array_index)))
  (if (>= (Utilities|Map|Length (Variables|Default|GetCheckRefP_Block)) 1)
    (CallFunction|SLGBlockInteract (Variables|Default|GetCheckRefP_Block))
    (Utilities|Map|Clear (Variables|Default|GetCheckRefP_Block))
    (return true)
    (else
      (return false))))

(fn SLGGetSpawnPosition
  (return 0))