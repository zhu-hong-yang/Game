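; Blueprint function library providing battle damage calculation and a restart of the current level.
; CalculateDamage rolls the attacker's ATN at 90–100% and adds weapon attack scaled by proficiency with its weapon type.
; A math expression reduces this by the target's DEF times a resistance chosen by the attacker's weapon type.
; Targets that are not MainBattleActors take the rolled attack plus unscaled weapon attack, without mitigation.
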(fn CalculateDamage
  (params (AttackActor :type Actor%20Object%20Reference) (DamageActor :type Actor%20Object%20Reference))
  (LocalVariables|SetActtackBA 0)
  (LocalVariables|SetDamageBA 0)
  (bind _asmain_battle_actor (Utilities|Casting|CastToMainBattleActor AttackActor))
  (LocalVariables|SetActtackBA _asmain_battle_actor)
  (bind _asmain_battle_actor_2 (Utilities|Casting|CastToMainBattleActor DamageActor)
    (:then
      (LocalVariables|SetDamageBA _asmain_battle_actor_2)
      (return (|((100/(100+(DEF*RA)))*(ATN+(WPATN*WP))) (Variables|/Game/HeroBP/BattleActor/MainBattleActor.MainBattleActor_C|GetDEF (LocalVariables|GetDamageBA)) (* (Utilities|Select :Index (Variables|/Game/HeroBP/BattleActor/MainBattleActor.MainBattleActor_C|GetWeaponType (LocalVariables|GetActtackBA)) :NewEnumerator18 (.SRA (Utilities|Struct|BreakRA_St (Variables|/Game/HeroBP/BattleActor/MainBattleActor.MainBattleActor_C|GetRA (LocalVariables|GetDamageBA)))) :NewEnumerator6 (.CRA (Utilities|Struct|BreakRA_St (Variables|/Game/HeroBP/BattleActor/MainBattleActor.MainBattleActor_C|GetRA (LocalVariables|GetDamageBA)))) :NewEnumerator7 (.SRA (Utilities|Struct|BreakRA_St (Variables|/Game/HeroBP/BattleActor/MainBattleActor.MainBattleActor_C|GetRA (LocalVariables|GetDamageBA)))) :NewEnumerator8 (.PRA (Utilities|Struct|BreakRA_St (Variables|/Game/HeroBP/BattleActor/MainBattleActor.MainBattleActor_C|GetRA (LocalVariables|GetDamageBA)))) :NewEnumerator9 (.PRA (Utilities|Struct|BreakRA_St (Variables|/Game/HeroBP/BattleActor/MainBattleActor.MainBattleActor_C|GetRA (LocalVariables|GetDamageBA)))) :NewEnumerator10 (.SRA (Utilities|Struct|BreakRA_St (Variables|/Game/HeroBP/BattleActor/MainBattleActor.MainBattleActor_C|GetRA (LocalVariables|GetDamageBA)))) :NewEnumerator11 (.ERA (Utilities|Struct|BreakRA_St (Variables|/Game/HeroBP/BattleActor/MainBattleActor.MainBattleActor_C|GetRA (LocalVariables|GetDamageBA)))) :NewEnumerator12 (.ERA (Utilities|Struct|BreakRA_St (Variables|/Game/HeroBP/BattleActor/MainBattleActor.MainBattleActor_C|GetRA (LocalVariables|GetDamageBA)))) :NewEnumerator13 (.BRA (Utilities|Struct|BreakRA_St (Variables|/Game/HeroBP/BattleActor/MainBattleActor.MainBattleActor_C|GetRA (LocalVariables|GetDamageBA)))) :NewEnumerator14 (.BRA (Utilities|Struct|BreakRA_St (Variables|/Game/HeroBP/BattleActor/MainBattleActor.MainBattleActor_C|GetRA (LocalVariables|GetDamageBA)))) :NewEnumerator15 (.SRA (Utilities|Struct|BreakRA_St (Variables|/Game/HeroBP/BattleActor/MainBattleActor.MainBattleActor_C|GetRA (LocalVariables|GetDamageBA))))) 0.01) (Math|Random|RandomFloatinRange (* (Variables|/Game/HeroBP/BattleActor/MainBattleActor.MainBattleActor_C|GetATN (LocalVariables|GetActtackBA)) 0.9) (Variables|/Game/HeroBP/BattleActor/MainBattleActor.MainBattleActor_C|GetATN (LocalVariables|GetActtackBA))) (* (Math|Conversions|ToInteger(Byte) (.Value (Utilities|Map|Find (Utilities|Struct|BreakWeaponProficiencySt (Variables|/Game/HeroBP/BattleActor/MainBattleActor.MainBattleActor_C|GetWeaponProficiency (LocalVariables|GetActtackBA))) (Variables|/Game/HeroBP/BattleActor/MainBattleActor.MainBattleActor_C|GetWeaponType (LocalVariables|GetActtackBA))))) 0.01) (Variables|/Game/HeroBP/BattleActor/MainBattleActor.MainBattleActor_C|GetWeaponATN (LocalVariables|GetActtackBA)))))
    (:CastFailed
      (return (+ (Math|Random|RandomFloatinRange (* (Variables|/Game/HeroBP/BattleActor/MainBattleActor.MainBattleActor_C|GetATN (LocalVariables|GetActtackBA)) 0.9) (Variables|/Game/HeroBP/BattleActor/MainBattleActor.MainBattleActor_C|GetATN (LocalVariables|GetActtackBA))) (Variables|/Game/HeroBP/BattleActor/MainBattleActor.MainBattleActor_C|GetWeaponATN (LocalVariables|GetActtackBA)))))))

(fn RestartLevel
  (bind _returnvalue (Game|GetCurrentLevelName 0))
  (Game|OpenLevel(byName) 0 (Utilities|String|StringToName _returnvalue))
  (return))