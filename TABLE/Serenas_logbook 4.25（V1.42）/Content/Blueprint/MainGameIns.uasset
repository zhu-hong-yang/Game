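; Game instance for an RPG, holding the hero roster, team slots, calendar and progression logic.
; Events remove heroes, total carried weight from data tables, advance the date, and reposition the player after map changes by door name or stored location.
; FucLevelUP scales EXP by level gap through FucGetExp, loops level-ups to a cap of 99, then recalculates HP/MP using gear bonuses from GetMaxHPMPFromGoods.
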(event Custom|UpdateHeroWeight
  (params (HeroName :type Name))
  (bind _playerheroname (Variables|PlayerInfo|GetPlayerHeroName))
  (bind _playerhero (Variables|PlayerInfo|GetPlayerHero))
  (bind _returnvalue (Utilities|Array|FindItem _playerheroname HeroName))
  (bind _output (Utilities|Array|Get(acopy) _playerhero _returnvalue))
  (bind (_heroid _heroname _level _exp _hp _mp _skill _weapon _hat _cloth _pant _shoes _item) (Utilities|Struct|BreakHeroMapping _output))
  ;[1 1 1] 更新单个角色负重
  (Variables|Math|SetRefFloat 0.0)
  (bind _returnvalue_2 (Utilities|GetDataTableRow "/Game/HeroInfo/HeroDT.HeroDT" _heroid)
    (:then
      (Utilities|Struct|SetmembersinHeroMapping _output (.MaxWeight (Utilities|Struct|BreakHeroStatSt _returnvalue_2)))
      (for _array_element _item
        (bind _returnvalue_3 (Utilities|GetDataTableRow "/Game/Item/AllGoodsDT.AllGoodsDT" (.ItemID (Utilities|Struct|BreakGoodsDataMapping _array_element)))
          (:then
            (Variables|Math|SetRefFloat (+ (Variables|Math|GetRefFloat) (* (Math|Conversions|ToInteger(Byte) (.Amount (Utilities|Struct|BreakGoodsDataMapping _array_element))) (.Weight (Utilities|Struct|BreakMainItemSt _returnvalue_3))))))))
      (Utilities|Struct|SetmembersinHeroMapping _output (Variables|Math|GetRefFloat)))))

(event Custom|DelectHeroEventDispatcher_Event
  (params (HeroName :type Name))
  (bind _playerheroname (Variables|PlayerInfo|GetPlayerHeroName))
  (bind _returnvalue (Utilities|Array|FindItem _playerheroname HeroName))
  ;[1 1 1] 删除角色事件
  (for _array_element (Variables|PlayerInfo|GetTeamSlot)
    (Utilities|Array|RemoveItem (Utilities|Struct|BreakHeroSlot _array_element) HeroName))
  (Utilities|Array|RemoveIndex (Variables|PlayerInfo|GetPlayerHero) _returnvalue)
  (Utilities|Array|RemoveIndex _playerheroname _returnvalue)
  (Default|CallDelectHeroEventDispatcher HeroName))

(event Custom|UpdateTeamWeight
  ;[1 1 1] 更新所有角色负重
  (for _array_element (Variables|PlayerInfo|GetPlayerHero)
    (Variables|Math|SetRefFloat 0.0)
    (bind _returnvalue (Utilities|GetDataTableRow "/Game/HeroInfo/HeroDT.HeroDT" (.HeroID (Utilities|Struct|BreakHeroMapping _array_element)))
      (:then
        (Utilities|Struct|SetmembersinHeroMapping _array_element (.MaxWeight (Utilities|Struct|BreakHeroStatSt _returnvalue)))
        (for _array_element_2 (.Item (Utilities|Struct|BreakHeroMapping _array_element))
          (bind _returnvalue_2 (Utilities|GetDataTableRow "/Game/Item/AllGoodsDT.AllGoodsDT" (.ItemID (Utilities|Struct|BreakGoodsDataMapping _array_element_2)))
            (:then
              (Variables|Math|SetRefFloat (+ (Variables|Math|GetRefFloat) (* (Math|Conversions|ToInteger(Byte) (.Amount (Utilities|Struct|BreakGoodsDataMapping _array_element_2))) (.Weight (Utilities|Struct|BreakMainItemSt _returnvalue_2))))))))
        (Utilities|Struct|SetmembersinHeroMapping _array_element (Variables|Math|GetRefFloat))))))

(event Custom|ChangeMapLoadDataEvent
  ;[1 1 1] 转换地图后的位置
  (if (Utilities|Name|Equal(Name) (Variables|Default|GetDoorName) "None")
    (if (Variables|Default|GetbTeleport)
      (Transformation|Teleport (Game|GetPlayerCharacter 0) (Variables|Default|GetTeleportLocation) "0, 0, 0")
      (Variables|Default|SetbTeleport false))
    (else
      (bind _outactors (Actor|GetAllActorsOfClass "/Game/RPGSystem/Room/EnterBuild.EnterBuild_C"))
      (bind _array_element (Utilities|Array|ForEachLoopwithBreak _outactors :!label _label)
        (:LoopBody
          (if (Utilities|Name|Equal(Name) (Variables|Default|GetDoorName) (Variables|/Game/RPGSystem/Room/EnterBuild.EnterBuild_C|GetDoorName _array_element))
            (Transformation|Teleport (Game|GetPlayerCharacter 0) (+ (.Location (Math|Transform|BreakTransform (Variables|/Game/RPGSystem/Room/EnterBuild.EnterBuild_C|GetEnterLocation _array_element))) (Transformation|GetActorLocation _array_element)) "0, 0, 0")
            (goto _label Break)))
        (:Completed
          (Variables|Default|SetDoorName "None"))))))

(event Custom|UpdateDate
  (if (> (Variables|Date|GetDay) (Math|Conversions|ToByte(Integer) (Class|KismetMathLibrary|DaysinMonth (Variables|Date|GetYear) (Math|Conversions|ToInteger(Byte) (Variables|Date|GetMonth)))))
    (Variables|Date|SetDay 1)
    (if (> (Variables|Date|GetMonth) 12)
      (Variables|Date|SetMonth 1)
      (Math|Integer|IncrementInt (Variables|Date|GetYear))
      (else
        (Variables|Date|SetMonth (+ (Variables|Date|GetMonth) 1))))
    (else
      (Variables|Date|SetDay (+ (Variables|Date|GetDay) 1)))))

(fn FucGetExp
  (params (ReComLevel :type Byte) (HeroLevel :type Byte) (GetExp :type Float%20%28single-precision%29))
  (bind _returnvalue (Math|Conversions|ToInteger(Byte) HeroLevel))
  (bind _returnvalue_2 (Math|Conversions|ToInteger(Byte) ReComLevel))
  (bind _levelgetexpmapping (Variables|EXP|GetLevelGetExpMapping))
  (bind _returnvalue_3 (- _returnvalue_2 _returnvalue))
  (if (<= _returnvalue_3 2)
    ;[1 1 1] 普通经验
    (LocalVariables|SetEXP GetExp)
    (return (LocalVariables|GetEXP))
    (else
      (bind _keys (Utilities|Map|Keys _levelgetexpmapping))
      (bind _arrayelement (Utilities|ReverseforEachLoopwithBreak _keys :!label _label)
        (:LoopBody
          (if (>= _returnvalue_3 _arrayelement)
            (goto _label Break)))
        (:Completed
          (LocalVariables|SetEXP (* (.Value (Utilities|Map|Find _levelgetexpmapping _arrayelement)) GetExp))
          (return (LocalVariables|GetEXP)))))))

(fn GetMaxHP/MPfromGoods
  (params (HeroMapping :type Hero%20Mapping%20Structure%20%28by%20ref%29))
  (bind (_heroid _heroname _level _exp _hp _mp _skill _weapon _hat _cloth _pant _shoes _item) (Utilities|Struct|BreakHeroMapping HeroMapping))
  (for _array_element (Utilities|Array|MakeArray _hat _cloth _pant _shoes)
    (bind _returnvalue (Utilities|GetDataTableRow "/Game/Item/EquipDataTable.EquipDataTable" _array_element)
      (:then
        (LocalVariables|SetRefLocalMaxHP (+ (LocalVariables|GetRefLocalMaxHP) (.MaxHP (Utilities|Struct|BreakStatSt (.Stat (Utilities|Struct|BreakMainItemSt _returnvalue))))))
        (LocalVariables|SetRefLocalMaxMP (+ (LocalVariables|GetRefLocalMaxMP) (.MaxMP (Utilities|Struct|BreakStatSt (.Stat (Utilities|Struct|BreakMainItemSt _returnvalue)))))))))
  (for _array_element_2 _item
    (bind _returnvalue_2 (Utilities|GetDataTableRow "/Game/Item/EquipDataTable.EquipDataTable" (.ItemID (Utilities|Struct|BreakGoodsDataMapping _array_element_2)))
      (:then
        (if (Utilities|Enum|Equal(Enum) (.GoodsType (Utilities|Struct|BreakMainItemSt _returnvalue_2)) "NewEnumerator21")
          (if (Utilities|Enum|Equal(Enum) (.ItemType (Utilities|Struct|BreakMainItemSt _returnvalue_2)) "NewEnumerator18")
            (LocalVariables|SetRefLocalMaxHP (+ (LocalVariables|GetRefLocalMaxHP) (.MaxHP (Utilities|Struct|BreakStatSt (.Stat (Utilities|Struct|BreakMainItemSt _returnvalue_2))))))
            (LocalVariables|SetRefLocalMaxMP (+ (LocalVariables|GetRefLocalMaxMP) (.MaxMP (Utilities|Struct|BreakStatSt (.Stat (Utilities|Struct|BreakMainItemSt _returnvalue_2)))))))))))
  (return (LocalVariables|GetRefLocalMaxHP) (LocalVariables|GetRefLocalMaxMP)))

(fn FucLevelUP
  (params (HeroName :type Name%20%28by%20ref%29) (ReComLevel :type Byte) (GetExp :type Float%20%28single-precision%29))
  (bind _playerhero (Variables|PlayerInfo|GetPlayerHero))
  (bind _playerheroname (Variables|PlayerInfo|GetPlayerHeroName))
  (bind _returnvalue (Utilities|Array|FindItem _playerheroname HeroName))
  (bind _output (Utilities|Array|Get(acopy) _playerhero _returnvalue))
  (bind (_heroid _heroname _level _exp) (Utilities|Struct|BreakHeroMapping _output))
  (bind _returnvalue_2 (Utilities|MacroGetExpNeed _level))
  (bind _returnvalue_3 (>= _exp _returnvalue_2))
  (bind _returnvalue_4 (Utilities|GetDataTableRow "/Game/HeroInfo/HeroDT.HeroDT" _heroid)
    (:then
      (LocalVariables|SetRefBeforeLevel _level)
      (bind _gaveexp (CallFunction|FucGetExp ReComLevel _level GetExp)) ; 计算获得经验
      (LocalVariables|SetRefExp _gaveexp)
      (Utilities|Struct|SetmembersinHeroMapping _output (+ _exp _gaveexp)) ; 写入经验
      (if _returnvalue_3 ; 判断是否升级
        (bind (_localmaxhp_fromgoods _localmaxmp_fromgoods) (CallFunction|GetMaxHP/MPfromGoods _output))
        (Variables|EXP|SetRefMaxHP_FromGoods _localmaxhp_fromgoods)
        (Variables|EXP|SetRefMaxMP_FromGoods _localmaxmp_fromgoods)
        (Variables|EXP|SetRefMaxHP (Utilities|MacroGetHeroStat (.MaxHP (Utilities|Struct|BreakHeroStatSt _returnvalue_4)) (.MaxHP (Utilities|Struct|BreakUpgradeData (.UpgradeStat (Utilities|Struct|BreakHeroStatSt _returnvalue_4)))) _level))
        (Variables|EXP|SetRefMaxMP (Utilities|MacroGetHeroStat (.MaxMP (Utilities|Struct|BreakHeroStatSt _returnvalue_4)) (.MaxMP (Utilities|Struct|BreakUpgradeData (.UpgradeStat (Utilities|Struct|BreakHeroStatSt _returnvalue_4)))) _level))
        (Variables|Math|SetLoopBreak true)
        (while (Variables|Math|GetLoopBreak)
          (if (< _level 99)
            (Utilities|Struct|SetmembersinHeroMapping _output (- _exp _returnvalue_2))
            (Utilities|Struct|SetmembersinHeroMapping _output (+ _level 1))
            (if (not _returnvalue_3)
              (Variables|Math|SetLoopBreak false))
            (else
              (Variables|Math|SetLoopBreak false))))
        (LocalVariables|SetRefNowLevel _level)
        (Utilities|Struct|SetmembersinHeroMapping _output (+ (/ (- (+ (.MaxHP (Utilities|Struct|BreakHeroStatSt _returnvalue_4)) (Variables|EXP|GetRefMaxHP_FromGoods)) (+ (Variables|EXP|GetRefMaxHP_FromGoods) (Variables|EXP|GetRefMaxHP))) (+ (Variables|EXP|GetRefMaxHP_FromGoods) (Variables|EXP|GetRefMaxHP))) (.HP (Utilities|Struct|BreakHeroStatSt _returnvalue_4))) (+ (/ (- (+ (.MaxMP (Utilities|Struct|BreakHeroStatSt _returnvalue_4)) (Variables|EXP|GetRefMaxMP_FromGoods)) (+ (Variables|EXP|GetRefMaxMP) (Variables|EXP|GetRefMaxMP_FromGoods))) (+ (Variables|EXP|GetRefMaxMP) (Variables|EXP|GetRefMaxMP_FromGoods))) (.MP (Utilities|Struct|BreakHeroStatSt _returnvalue_4))))
        (return (LocalVariables|GetRefExp) (LocalVariables|GetRefBeforeLevel) (LocalVariables|GetRefNowLevel))
        (else
          (return (LocalVariables|GetRefExp) (LocalVariables|GetRefBeforeLevel) (LocalVariables|GetRefBeforeLevel)))))))