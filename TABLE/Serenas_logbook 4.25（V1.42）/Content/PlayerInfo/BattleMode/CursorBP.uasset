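; CursorBP is a battle-mode cursor actor that keeps a cone marker floating just above whatever surface or object lies at its position.
; Each tick it line-traces vertically through its location against static, dynamic and pawn objects, setting the cone's relative height slightly above the hit, or to a default offset without one.
; The trace draws debug lines every frame, and the construction script tints the cone blue through a material parameter.
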(event EventBeginPlay)

(event EventTick
  (params (DeltaSeconds :type Float%20%28single-precision%29))
  (bind _returnvalue (Transformation|GetActorLocation))
  (bind (_outhit _returnvalue_2) (Collision|LineTraceForObjects (+ _returnvalue "0, 0,500.000000") (- _returnvalue "0, 0,500.000000") (Utilities|Array|MakeArray "ObjectTypeQuery1" "ObjectTypeQuery2" "ObjectTypeQuery3") false 0 "ForOneFrame"))
  (if _returnvalue_2
    (Transformation|SetRelativeLocation (Variables|Default|GetCone) (Math|Vector|MakeVector 0.0 0.0 (+ (.Z (Math|Vector|BreakVector (- (.Location (Collision|BreakHitResult _outhit)) (Transformation|GetActorLocation)))) 5e+01)) false false)
    (else
      (Transformation|SetRelativeLocation (Variables|Default|GetCone) (Math|Vector|MakeVector 0.0 0.0 5e+01) false false))))

(fn ConstructionScript
  (Rendering|Material|SetVectorParameterValueonMaterials (Variables|Default|GetCone) "Color" (Math|Conversions|ToVector(LinearColor) "(R=0.245097,G=0.363373,B=1.000000,A=1.000000)")))