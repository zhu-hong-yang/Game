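; InteractNPC_BP is an interactable RPG NPC that can move the player to another level when its dialogue ends.
; After the parent's dialogue-end logic, it looks up the game instance's current Chapter in its LevelName map.
; On a match, it locks the player through MainRPG_PlayerController and shows a fade widget.
; It waits for the length of the widget's FadeOut animation, then opens the mapped level.
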(event EventBeginPlay)

(event Collision|EventActorBeginOverlap
  (params (OtherActor :type Actor%20Object%20Reference))
  (|CallParentFunction OtherActor) ; 此节点被禁用，将不会被调用。\n从引脚连出引线来编译功能。
)

(event EventTick
  (params (DeltaSeconds :type Float%20%28single-precision%29))
  (|CallParentFunction DeltaSeconds) ; 此节点被禁用，将不会被调用。\n从引脚连出引线来编译功能。
)

(event EventRPGDialogueEnd
  (bind _levelname (Variables|Default|GetLevelName))
  (bind _gameins (Variables|Default|GetGameIns))
  (bind _chapter (Variables|/Game/Blueprint/MainGameIns.MainGameIns_C|GetChapter _gameins))
  (bind (_value _returnvalue) (Utilities|Map|Find _levelname _chapter))
  (|CallParentFunction)
  (if _returnvalue
    (bind _asmain_rpg_player_controller (Utilities|Casting|CastToMainRPG_PlayerController (Game|GetPlayerController 0)))
    (Variables|/Game/PlayerInfo/RPG_Mode/MainRPG_PlayerController.MainRPG_PlayerController_C|SetLockPlayer _asmain_rpg_player_controller true)
    (bind _returnvalue_2 (UserInterface|CreateWidget "/Game/UMG/FadeInOrOutWG.FadeInOrOutWG_C" 0 true))
    (UserInterface|Viewport|AddtoViewport _returnvalue_2 20)
    (Utilities|FlowControl|Delay (Class|WidgetAnimation|GetEndTime (Variables|/Game/UMG/FadeInOrOutWG.FadeInOrOutWG_C|GetFadeOut _returnvalue_2)))
    (Game|OpenLevel(byName) _value)))

(fn ConstructionScript
  (|CallParentFunction))