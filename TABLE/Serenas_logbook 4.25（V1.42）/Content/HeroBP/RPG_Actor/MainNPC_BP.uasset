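; Main NPC Blueprint that the player interacts with to start a dialogue chosen by story chapter.
; If no start row is set, it picks one by the GameInstance chapter, falling back through a reverse search to earlier chapters.
; Interaction opens or advances dialogue through HUD interface messages and turns the NPC toward the player once, restoring rotation when dialogue ends.
; A CanInteract flag gates interaction and the dialogue icon.
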(event EventBeginPlay
  (bind _asmain_game_ins (Utilities|Casting|CastToMainGameIns (Game|GetGameInstance)))
  (Variables|Default|SetGameIns _asmain_game_ins))

(event Collision|EventActorBeginOverlap
  (params (OtherActor :type Actor%20Object%20Reference)))

(event EventRPGDialogueEnd
  ;[1 1 1] 对话之后
  (Variables|/Game/PlayerInfo/RPG_Mode/MainRPG_Character2D.MainRPG_Character2D_C|SetRefInteracting (Variables|Default|GetMainRPG_PlayerCharacter) 0)
  (Variables|Default|SetMainRPG_PlayerCharacter 0)
  (Transformation|SetActorRotation (Variables|Default|GetRefDefaultRotation))
  (Utilities|FlowControl|Delay 0.0)
  ;[1 1 1] 创建对话
  (Utilities|FlowControl|DoOnce false) ; enters at Reset
)

(event EventRPGShowInteractIcon
  (params (Show :type Boolean))
  ;[1 1 1] 显示互动图标
  (if (Variables|Default|GetCanInteract)
    (Development|SetHiddeninGame (Variables|Default|GetDialogueIcon) (not Show) false)))

(event EventTick
  (params (DeltaSeconds :type Float%20%28single-precision%29))
  (|CallParentFunction DeltaSeconds))

(event EventRPGInteractEvent
  (params (Actor :type Actor%20Object%20Reference))
  (bind _returnvalue (Game|GetPlayerController 0))
  (bind _chapter (Variables|Default|GetChapter))
  (bind _gameins (Variables|Default|GetGameIns))
  (bind _returnvalue_2 (HUD|GetHUD _returnvalue))
  (bind _chapter_2 (Variables|/Game/Blueprint/MainGameIns.MainGameIns_C|GetChapter _gameins))
  (bind _returnvalue_3 (Utilities|Array|FindItem _chapter _chapter_2))
  ;[1 1 1] 创建对话
  (if (Variables|Default|GetCanInteract)
    (if (Utilities|Name|Equal(Name) (Variables|Default|GetRowNameStart) "None")
      ;;[1 1 1] 设置段落
      (if (== _returnvalue_3 -1)
        (bind (_arrayindex _arrayelement) (Utilities|ReverseforEachLoopwithBreak _chapter :!label _label)
          (:LoopBody
            (Variables|Default|SetRowNameStart (Utilities|String|StringToName (Utilities|Array|Get(acopy) (Variables|Default|GetSelectDialogue) _arrayindex)))
            (if (>= _chapter_2 _arrayelement)
              (goto _label Break)))
          (:Completed
            (Utilities|FlowControl|Sequence :!label _label_2
              (:then_0
                (Utilities|IsValid (Variables|Default|GetMainRPG_PlayerCharacter)
                  (:Is%20Valid
                    _)
                  (:Is%20Not%20Valid
                    (bind _asmain_rpg_character_2d (Utilities|Casting|CastToMainRPG_Character2D (Game|GetPlayerCharacter 0)))
                    (Variables|Default|SetMainRPG_PlayerCharacter _asmain_rpg_character_2d)))
                (bind _isvisible (Class|RPGInteractInterface|RPGIsDialogueVisible(Message) (HUD|GetHUD (Game|GetPlayerController 0))))
                (if _isvisible
                  (Class|RPGInteractInterface|RPGInteractEvent(Message) _returnvalue_2)
                  (else
                    (Class|RPGInteractInterface|RPGSetUpDialogue(Message) _returnvalue_2 0 self))))
              (:then_1
                (Utilities|FlowControl|DoOnce false
                  (:Completed
                    (Variables|Default|SetRefDefaultRotation (Transformation|GetActorRotation))
                    (Transformation|SetActorRotation (Math|Rotator|MakeRotator 0.0 0.0 (.yaw (Math|Rotator|FindLookatRotation (Transformation|GetActorLocation) (Transformation|GetActorLocation (Variables|Default|GetMainRPG_PlayerCharacter))))))))))))
        (else
          (Variables|Default|SetRowNameStart (Utilities|String|StringToName (Utilities|Array|Get(acopy) (Variables|Default|GetSelectDialogue) _returnvalue_3)))
          (goto _label_2)))
      (else
        (goto _label_2)))))

(fn ConstructionScript)

(fn RPGCheckCanInteract
  (return (Variables|Default|GetCanInteract)))

(fn RPGIsDialogueVisible
  (return false))