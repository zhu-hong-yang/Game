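; MainHeroBP is a hero character Blueprint that shows a 2D flipbook sprite in a 3D world, billboarded toward the player camera.
; Each Tick it yaws the sprite to the camera, with a clamped roll derived from the camera's pitch.
; The camera's yaw relative to the actor's rotation selects one of four directional flipbooks from AllAxisAnimation.
; On a direction change it swaps flipbooks while preserving playback position, so the animation continues seamlessly.
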(event EventTick
  (params (DeltaSeconds :type Float%20%28single-precision%29))
  (bind _returnvalue (Transformation|GetActorLocation))
  (bind _returnvalue_2 (Game|GetPlayerCameraManager 0))
  (bind _sprite (Variables|Default|GetSprite))
  (bind _allaxisanimation (Variables|Default|GetAllAxisAnimation))
  (bind (_loop _happenframe _up _down _left _right) (Utilities|Struct|BreakHeroAnimAxisAndEventSt _allaxisanimation))
  (bind _returnvalue_3 (Camera|GetCameraLocation _returnvalue_2))
  (bind _returnvalue_4 (Math|Rotator|FindLookatRotation _returnvalue _returnvalue_3))
  (bind (_roll _pitch _yaw) (Math|Rotator|BreakRotator _returnvalue_4))
  ;[1 1 1] 角色看向的位置
  (Transformation|SetWorldRotation (Variables|Default|GetSprite) (Math|Rotator|MakeRotator (Math|Float|Clamp(Float) (- 3.6e+02 _pitch) 3.4e+02 3.6e+02) 0.0 (- _yaw 9e+01)) false false)
  (Variables|Default|SetFaceToIndex (/ (+ (Math|Float|Truncate (+ (.Yaw (Math|Rotator|BreakRotator (Math|Rotator|Delta(Rotator) _returnvalue_4 (Transformation|GetActorRotation)))) 1.8e+02)) 45) (/ 360 4)))
  (if (not (== (Variables|Default|GetRefAnimation) (Utilities|Select :Index (Variables|Default|GetFaceToIndex) :Option%200 _up :Option%201 _left :Option%202 _down :Option%203 _right :Option%204 _up)))
    (Variables|Default|SetLocalFloat (Components|Timeline|GetPlaybackPosition _sprite))
    (Variables|Default|SetRefAnimation (Utilities|Select :Index (Variables|Default|GetFaceToIndex) :Option%200 _up :Option%201 _left :Option%202 _down :Option%203 _right :Option%204 _up))
    (Sprite|SetFlipbook (Variables|Default|GetSprite) (Variables|Default|GetRefAnimation))
    (Components|Timeline|SetPlaybackPosition _sprite (Variables|Default|GetLocalFloat) false)))

(fn ConstructionScript)