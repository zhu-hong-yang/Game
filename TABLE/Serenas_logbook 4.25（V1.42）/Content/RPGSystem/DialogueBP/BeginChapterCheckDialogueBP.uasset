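; Dialogue actor that auto-plays a story chapter's dialogue at level start, skipping chapters already read in that level.
; On BeginPlay it finds the current chapter's DataTable, checks the GameInstance's read record, then sends the table to the HUD and becomes the player's interaction target.
; RPGDialogueEnd clears that target and records the chapter under the level name, using parallel DialogueMap and DialogueCheck collections.
; Its interact-check and visibility functions always return false.
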(event EventBeginPlay
  (Utilities|FlowControl|Delay 0.0)
  (bind _asmain_rpg_player_controller (Utilities|Casting|CastToMainRPG_PlayerController (Game|GetPlayerController 0)))
  (Variables|Default|SetRefPlayerController _asmain_rpg_player_controller)
  (bind _asmain_game_ins (Utilities|Casting|CastToMainGameIns (Game|GetGameInstance)))
  (Variables|Default|SetMainGameIns _asmain_game_ins)
  ;[1 1 1] 这章节含有剧情
  (if (.ReturnValue (Utilities|Map|Find (Variables|Default|GetChapterDataTable) (Variables|/Game/Blueprint/MainGameIns.MainGameIns_C|GetChapter (Variables|Default|GetMainGameIns))))
    (bind _returnvalue (Game|GetCurrentLevelName true))
    ;[1 1 1] 是否读过
    (if (Utilities|Array|ContainsItem (Variables|/Game/Blueprint/MainGameIns.MainGameIns_C|GetDialogueMap (Variables|Default|GetMainGameIns)) _returnvalue)
      (if (not (Utilities|Array|ContainsItem (Utilities|Struct|BreakDialogueCheckSt (Utilities|Array|Get(acopy) (Variables|/Game/Blueprint/MainGameIns.MainGameIns_C|GetDialogueCheck (Variables|Default|GetMainGameIns)) (Utilities|Array|FindItem (Variables|/Game/Blueprint/MainGameIns.MainGameIns_C|GetDialogueMap (Variables|Default|GetMainGameIns)) _returnvalue))) (Variables|/Game/Blueprint/MainGameIns.MainGameIns_C|GetChapter (Variables|Default|GetMainGameIns))))
        (Class|RPGInteractInterface|RPGSetUpDialogue(Message) (HUD|GetHUD (Game|GetPlayerController 0)) (.Value (Utilities|Map|Find (Variables|Default|GetChapterDataTable) (Variables|/Game/Blueprint/MainGameIns.MainGameIns_C|GetChapter (Variables|Default|GetMainGameIns)))) self :!label _label)
        (Variables|/Game/PlayerInfo/RPG_Mode/MainRPG_Character2D.MainRPG_Character2D_C|SetRefInteracting (Variables|/Game/PlayerInfo/RPG_Mode/MainRPG_PlayerController.MainRPG_PlayerController_C|GetRefPlayerCharacter (Variables|Default|GetRefPlayerController)) self))
      (else
        (goto _label)))))

(event Collision|EventActorBeginOverlap
  (params (OtherActor :type Actor%20Object%20Reference)))

(event EventRPGDialogueEnd
  (bind _maingameins (Variables|Default|GetMainGameIns))
  (bind _maingameins_2 (Variables|Default|GetMainGameIns))
  (bind _chapter (Variables|/Game/Blueprint/MainGameIns.MainGameIns_C|GetChapter _maingameins_2))
  (bind _dialoguemap (Variables|/Game/Blueprint/MainGameIns.MainGameIns_C|GetDialogueMap _maingameins))
  (bind _dialoguecheck (Variables|/Game/Blueprint/MainGameIns.MainGameIns_C|GetDialogueCheck _maingameins))
  ;[1 1 1] 读完章节后写入
  (Variables|/Game/PlayerInfo/RPG_Mode/MainRPG_Character2D.MainRPG_Character2D_C|SetRefInteracting (Variables|/Game/PlayerInfo/RPG_Mode/MainRPG_PlayerController.MainRPG_PlayerController_C|GetRefPlayerCharacter (Variables|Default|GetRefPlayerController)) 0)
  (bind _returnvalue (Game|GetCurrentLevelName true))
  (if (Utilities|Array|ContainsItem _dialoguemap _returnvalue)
    (Utilities|Array|Add (Utilities|Struct|BreakDialogueCheckSt (Utilities|Array|Get(acopy) _dialoguecheck (Utilities|Array|FindItem _dialoguemap _returnvalue))) _chapter)
    (else
      (Utilities|Array|Add _dialoguemap _returnvalue)
      (Utilities|Array|Add _dialoguecheck (Utilities|Struct|MakeDialogueCheckSt (Utilities|Array|MakeArray _chapter))))))

(event EventRPGInteractEvent
  (params (Actor :type Actor%20Object%20Reference))
  (Class|RPGInteractInterface|RPGInteractEvent(Message) (HUD|GetHUD (Game|GetPlayerController 0))))

(event EventTick
  (params (DeltaSeconds :type Float%20%28single-precision%29)))

(fn ConstructionScript)

(fn RPGCheckCanInteract
  (return false))

(fn RPGIsDialogueVisible
  (return false))