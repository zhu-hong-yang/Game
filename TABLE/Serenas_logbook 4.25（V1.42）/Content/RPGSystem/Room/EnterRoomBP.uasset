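; EnterRoomBP is a room doorway trigger actor that toggles the visibility of a configurable set of objects as the player passes through.
; When the player character leaves the Box, its offset is unrotated into the actor's local space to find the exit side.
; Exiting on the negative X side shows the HiddenObject actors, while the other side hides them.
; The Construction Script sizes the Box from an extent variable.
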(event OnComponentEndOverlap(Box)
  (params (OverlappedComponent :type Primitive%20Component%20Object%20Reference) (OtherActor :type Actor%20Object%20Reference) (OtherComp :type Primitive%20Component%20Object%20Reference) (OtherBodyIndex :type Integer))
  (if (== OtherActor (Game|GetPlayerCharacter 0))
    (bind _result (Utilities|Set|ToArray (Variables|Default|GetHiddenObject)))
    (if (< (.X (Math|Vector|BreakVector (Math|Vector|UnrotateVector (- (Transformation|GetActorLocation OtherActor) (Transformation|GetActorLocation)) (Transformation|GetActorRotation)))) 0.0)
      (Rendering|SetActorHiddenInGame _result false)
      (else
        (Rendering|SetActorHiddenInGame _result true)))))

(event EventBeginPlay
  (Utilities|Set|ToArray (Variables|Default|GetHiddenObject)))

(event Collision|EventActorBeginOverlap
  (params (OtherActor :type Actor%20Object%20Reference)))

(event EventTick
  (params (DeltaSeconds :type Float%20%28single-precision%29)))

(fn ConstructionScript
  (Components|Box|SetBoxExtent (Variables|Default|GetBox) (Variables|Default|Get盒体范围) true))